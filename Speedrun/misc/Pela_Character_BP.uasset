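; Pelagornis character for a Speedrun mode: a rideable seabird that spawns saddled and allows a mounted fishing rod while swimming.
; Tick starts a kill timer whenever it is unridden, broadcasts a server warning near expiry, and cancels it on mounting.
; Tick also moves surplus raw fish meat to the speedrun rider.
; Non-dedicated instances add splash and water-trail effects, with local third-person camera interpolation for fishing.
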(event Custom|KillUnridden
  (bind _self self)
  ;[1 1 1] From Saber
  (Game|Damage|ApplyDamage _self 9999.0 0 _self "/Game/PrimalEarth/CoreBlueprints/DamageTypes/DmgType_Direct.DmgType_Direct_C"))

(event Custom|ReceiveTick_Copy
  (params (DeltaSeconds :type Float%20%28single-precision%29))
  ;[1 1 1] From Saber
)

(event EventTick
  (params (DeltaSeconds :type Float%20%28single-precision%29))
  (bind _returnvalue (Class|KismetSystemLibrary|GetTimerRemainingTime 0 "KillUnridden"))
  (bind _returnvalue_2 (Transformation|GetActorTransform))
  (bind _default (CallFunction|GetDefaultPela))
  (bind _watertrailparticle (Variables|Default|GetWaterTrailParticle))
  (bind _rider (Variables|Default|GetRider))
  (bind _myinventorycomponent (Variables|Default|GetMyInventoryComponent))
  (bind _charactermovement (Variables|Character|GetCharacterMovement))
  (bind (_location _rotation) (Math|Transform|BreakTransform _returnvalue_2))
  (bind _velocity (Variables|/Script/Engine.MovementComponent|GetVelocity _charactermovement))
  (bind _tpvcameraoffset (Variables|/Script/ShooterGame.PrimalCharacter|GetTPVCameraOffset _default))
  (bind _movementmode (Variables|/Script/Engine.CharacterMovementComponent|GetMovementMode _charactermovement))
  (bind _returnvalue_3 (Math|Vector|VectorLength _velocity))
  (bind _returnvalue_4 (Utilities|Enum|Equal(Enum) _movementmode "MOVE_Swimming"))
  (bind _returnvalue_5 (> _returnvalue_3 2e+02))
  (bind _returnvalue_6 (and _returnvalue_5 _returnvalue_4))
  (Utilities|FlowControl|Sequence
    (:then_0
      (if (not (Networking|IsDedicatedServer))
        (if (Class|PrimalCharacter|IsAlive)
          (Utilities|FlowControl|Sequence
            (:then_0
              (if (or (and (Utilities|Enum|Equal(Enum) (Variables|Default|GetLastMovementMode) "MOVE_Falling") _returnvalue_4) (and (Utilities|Enum|Equal(Enum) (Variables|Default|GetLastMovementMode) "MOVE_Swimming") (Utilities|Enum|Equal(Enum) _movementmode "MOVE_Flying")))
                (Game|SpawnActorfromClass (Variables|Default|GetSplashEmitter) (Math|Transform|MakeTransform (+ _location "0, 0,-90.000000") _rotation) true)))
            (:then_1
              (Variables|Default|SetLastMovementMode _movementmode))
            (:then_2
              (if (Math|Boolean|NotEqual(Boolean) (Variables|Default|GetbParticlesActivated) _returnvalue_6)
                (Variables|Default|SetbParticlesActivated _returnvalue_6)
                (if (Variables|Default|GetbParticlesActivated)
                  (Components|Activation|Activate _watertrailparticle true)
                  (else
                    (Components|Activation|Deactivate _watertrailparticle)))))
            (:then_3
              (if (Pawn|IsLocallyControlled)
                (if (Variables|Default|GetbHasRider)
                  (Utilities|IsValid _rider
                    (:Is%20Valid
                      (if (Class|Actor|BPIsA (Variables|/Script/ShooterGame.ShooterCharacter|GetCurrentWeapon _rider) "/Game/PrimalEarth/CoreBlueprints/Weapons/WeapFishingRod.WeapFishingRod_C")
                        (CallFunction|InterpCameraTPV (+ (Variables|Default|GetFishingTPVCameraOffset) _tpvcameraoffset) DeltaSeconds)
                        (else
                          (CallFunction|InterpCameraTPV _tpvcameraoffset DeltaSeconds))))))))))))
    (:then_1
      ;[1 1 1] From Saber
      (if (Variables|Default|GetbHasRider)
        (Utilities|Time|ClearTimerbyFunctionName 0 "KillUnridden")
        (goto _label Reset)
        (else
          (Utilities|FlowControl|Sequence
            (:then_0
              (Utilities|FlowControl|DoOnce false :!label _label
                (:Completed
                  (Utilities|Time|SetTimerbyFunctionName 0 "KillUnridden" 45.0))))
            (:then_1
              (Development|PrintString (Utilities|String|ToString(Float) _returnvalue) false false)
              (if (> 1e+01 _returnvalue)
                (Utilities|FlowControl|DoOnce false :!label _label_2
                  (:Completed
                    (bind _asshootergamemode (Utilities|Casting|CastToShooterGameMode (Game|GetGameMode)))
                    (Class|ShooterGameMode|SendServerNotification _asshootergamemode "Pelagornis will be killed unless ridden!" "(R=1.000000,G=1.000000,B=1.000000,A=1.000000)" 1.0 1e+01 0 0 -1 -1 false)))
                (elif (> _returnvalue 1e+01)
                  (goto _label_2 Reset))))))))
    (:then_2
      (bind _asplayerpawntest_speedrun_c (Utilities|Casting|CastToPlayerPawnTest_Speedrun (Variables|Default|GetRider)))
      (bind _returnvalue_7 (Class|PrimalInventoryComponent|GetItemTemplateQuantity _myinventorycomponent "/Game/PrimalEarth/CoreBlueprints/Items/Consumables/PrimalItemConsumable_RawMeat_Fish.PrimalItemConsumable_RawMeat_Fish_C" 0 true false false))
      (if (> _returnvalue_7 1)
        (Class|PrimalInventoryComponent|BPIncrementItemTemplateQuantity _myinventorycomponent "/Game/PrimalEarth/CoreBlueprints/Items/Consumables/PrimalItemConsumable_RawMeat_Fish.PrimalItemConsumable_RawMeat_Fish_C" (* (- _returnvalue_7 1) -1) true false true false false false)
        (Class|PrimalInventoryComponent|BPIncrementItemTemplateQuantity (Variables|/Game/Mods/Speedrun/PlayerPawnTest_Speedrun.PlayerPawnTest_Speedrun_C|GetPrimalInventory1 _asplayerpawntest_speedrun_c) "/Game/PrimalEarth/CoreBlueprints/Items/Consumables/PrimalItemConsumable_RawMeat_Fish.PrimalItemConsumable_RawMeat_Fish_C" (- _returnvalue_7 1) true false true false false false)))))

(event EventBeginPlay
  ;[1 1 1] From Saber
  (Utilities|FlowControl|Delay 0.2)
  (Class|PrimalItem|AddNewItem "/Game/PrimalEarth/CoreBlueprints/Items/Armor/Saddles/PrimalItemArmor_PelaSaddle.PrimalItemArmor_PelaSaddle_C" (Variables|Default|GetMyInventoryComponent) true false 0.0 false 1 false 0.0 false))

(fn ConstructionScript
  (|CallParentFunction))

(fn InterpCameraTPV
  (params (targetOffset :type Vector) (deltaTime :type Float%20%28single-precision%29))
  (if (!= (Variables|Default|GetTPVCameraOffset) targetOffset)
    (if (Utilities|AreVectorsNearlyEqual (Variables|Default|GetTPVCameraOffset) targetOffset 0.5)
      (Variables|Default|SetTPVCameraOffset targetOffset)
      (else
        (Variables|Default|SetTPVCameraOffset (Math|Interpolation|VInterpTo (Variables|Default|GetTPVCameraOffset) targetOffset deltaTime (Variables|Default|GetInterpCameraSpeed)))))))

(fn BPNotifyClearRider
  (params (RiderClearing :type Shooter%20Character%20Object%20Reference))
  (|CallParentFunction RiderClearing)
  (Variables|Default|SetTPVCameraOffset (Variables|/Script/ShooterGame.PrimalCharacter|GetTPVCameraOffset (CallFunction|GetDefaultPela))))

(fn GetDefaultPela
  (bind _returnvalue (Class|VictoryCore|GetDefaultObject self))
  (bind _aspela_character_bp_c (Utilities|Casting|CastToPela_Character_BP _returnvalue))
  (return _aspela_character_bp_c))

(fn BPForceAllowMountedWeapon
  (params (WeaponTemplate :type Shooter%20Weapon%20Class%20Reference))
  (return (and (Utilities|Enum|Equal(Enum) (Variables|/Script/Engine.CharacterMovementComponent|GetMovementMode (Variables|Character|GetCharacterMovement)) "MOVE_Swimming") (Utilities|ClassIsChildOf WeaponTemplate "/Game/PrimalEarth/CoreBlueprints/Weapons/WeapFishingRod.WeapFishingRod_C"))))